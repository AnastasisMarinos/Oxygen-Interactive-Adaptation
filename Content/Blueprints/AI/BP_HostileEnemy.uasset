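; BP_HostileEnemy is a hostile AI enemy that faces the player and alternates in and out of attacking.
; On BeginPlay it caches the player character and starts two looping timers.
; A fast LookAtPlayer timer smoothly interpolates the actor's rotation toward the player, standing in for Tick.
; A slower AttackPlayer timer flips ChasingPlayer and writes the bShouldAttack Blackboard key on its AI controller.
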(event `self.ReceiveBeginPlay`
  (bind _asbp_player_character (cast `/Game/Blueprints/Player/BP_PlayerCharacter` (`GameplayStatics.GetPlayerCharacter` 0)))
  (set `self.PlayerReference` _asbp_player_character)
  (`KismetSystemLibrary.K2_SetTimer` null "LookAtPlayer" 0.01 true)
  (`KismetSystemLibrary.K2_SetTimer` null "AttackPlayer" 4.0 true))

(fn `AttackPlayer`
  (bind _returnvalue (`AIBlueprintHelperLibrary.GetBlackboard` (`AIBlueprintHelperLibrary.GetAIController` self)))
  (if (`self.ChasingPlayer?`)
    (`BlackboardComponent.SetValueAsBool` _returnvalue "bShouldAttack" false)
    (set `self.ChasingPlayer?` false)
    (else
      (`BlackboardComponent.SetValueAsBool` _returnvalue "bShouldAttack" true)
      (set `self.ChasingPlayer?` true))))

(fn `LookAtPlayer`
  (`self.K2_SetActorRotation` (`KismetMathLibrary.RInterpTo` (`self.K2_GetActorRotation`) (`KismetMathLibrary.FindLookAtRotation` (`self.K2_GetActorLocation`) (`self.K2_GetActorLocation` (`self.PlayerReference`))) (`GameplayStatics.GetWorldDeltaSeconds`) 5.0)))

(fn `UserConstructionScript`)