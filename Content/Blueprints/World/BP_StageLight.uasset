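; Moving-head stage light whose yoke and head swing to random angles and which can strobe, driven by LightingTimerManager time broadcasts.
; Each broadcast picks new yaw and roll targets, which two looping timers ease toward with FInterpTo.
; StrobeLight toggles spot intensity and head emissive, with InverseStrobe flipping the spot's phase relative to the emissive.
; Game end changes the manager's time signature and sets rotation speed.
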(event `self.ReceiveBeginPlay`
  (`KismetSystemLibrary.K2_SetTimer` null "RotateYoke" 0.02 true)
  (`KismetSystemLibrary.K2_SetTimer` null "RotateHead" 0.02 true)
  (`LightingTimerManager.SetTimeSignature` (`self.LightingTimerManager`) 2.0))

(event `self.LightingTimerManager.OnTimeBroadcast`
  (params (bShouldStrobe :type Boolean))
  (`self.RandomYokeRotation`)
  (`self.RandomHeadRotation`)
  (if bShouldStrobe
    (`self.StrobeLight`)))

(event `OnGameEnd`
  (`LightingTimerManager.SetTimeSignature` (`self.LightingTimerManager`) 4.0)
  (set `self.LightRotationSpeed` 1.0))

(fn `RandomHeadRotation`
  (set `self.HeadRotationTarget` (`KismetMathLibrary.RandomFloatInRange` -55.0 55.0)))

(fn `RandomYokeRotation`
  (set `self.YokeRotationTarget` (`KismetMathLibrary.RandomFloatInRange` -180.0 180.0)))

(fn `RotateHead`
  (bind _sm_lighthead (`self.SM_LightHead`))
  (bind _relativerotation_roll (`KismetMathLibrary.BreakRotator` (`SceneComponent.RelativeRotation` _sm_lighthead)))
  (`SceneComponent.K2_SetRelativeRotation` _sm_lighthead (`KismetMathLibrary.MakeRotator` (`KismetMathLibrary.FInterpTo` _relativerotation_roll (`self.HeadRotationTarget`) (`GameplayStatics.GetWorldDeltaSeconds`) (`self.LightRotationSpeed`))) false false))

(fn `RotateYoke`
  (bind _sm_lightyoke (`self.SM_LightYoke`))
  (bind (_relativerotation_roll _relativerotation_pitch _relativerotation_yaw) (`KismetMathLibrary.BreakRotator` (`SceneComponent.RelativeRotation` _sm_lightyoke)))
  (`SceneComponent.K2_SetRelativeRotation` _sm_lightyoke (`KismetMathLibrary.MakeRotator` 0.0 0.0 (`KismetMathLibrary.FInterpTo` _relativerotation_yaw (`self.YokeRotationTarget`) (`GameplayStatics.GetWorldDeltaSeconds`) (`self.LightRotationSpeed`))) false false))

(fn `StrobeLight`
  (bind _spotlight (`self.SpotLight`))
  (bind _sm_lighthead (`self.SM_LightHead`))
  (if (`self.InverseStrobe`)
    (if (`self.IsLightOn`)
      (`LightComponent.SetIntensity` _spotlight 0.0)
      (set `self.IsLightOn` false)
      (`MeshComponent.SetScalarParameterValueOnMaterials` _sm_lighthead "Emission" 0.1 :!label _label)
      (else
        (`LightComponent.SetIntensity` _spotlight (`self.DefaultLightIntensity`))
        (set `self.IsLightOn` true)
        (`MeshComponent.SetScalarParameterValueOnMaterials` _sm_lighthead "Emission" 15.0 :!label _label_2)))
    (elif (`self.IsLightOn`)
      (`LightComponent.SetIntensity` _spotlight (`self.DefaultLightIntensity`))
      (set `self.IsLightOn` false)
      (goto _label)
      (else
        (`LightComponent.SetIntensity` _spotlight 0.0)
        (set `self.IsLightOn` true)
        (goto _label_2)))))

(fn `UserConstructionScript`
  (`LightComponent.SetIntensity` (`self.SpotLight`) (`self.DefaultLightIntensity`)))