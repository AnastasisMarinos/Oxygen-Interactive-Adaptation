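; BP_WordInteractable is a world actor that displays its Keyword as particle text lit by a spotlight, themed to the audio line colors.
; On BeginPlay it passes the Keyword into the particle text parameter and creates a dynamic material instance on the text.
; The particle color and spotlight color both come from the AudioManager's next line theme color.
; No interaction logic appears in its graphs.
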(event `self.ReceiveBeginPlay`
  (bind _returnvalue (`AudioManager.GetNextLineThemeColor` (`self.AudioManager`)))
  (`ParticleTextParamComponent.SetParamText` (`self.ParticleTextParam`) (`KismetTextLibrary.Conv_TextToString` (`self.Keyword`)))
  (bind _returnvalue_2 (`PrimitiveComponent.CreateDynamicMaterialInstance` (`self.P_TEXT`) 0 "/Game/Assets/Particles/Text/M_PARTICLE.M_PARTICLE" "None"))
  (`MaterialInstanceDynamic.SetVectorParameterValue` _returnvalue_2 "ParticleColor" _returnvalue)
  (`LightComponent.SetLightColor` (`self.SpotLight`) _returnvalue true))

(fn `UserConstructionScript`)