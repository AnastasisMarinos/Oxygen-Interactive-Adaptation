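; BP_CeilingLights is a world ceiling light whose strobe material is timed to a beat interval.
; SetStrobeTime divides the given strobe time by the LightingTimerManager's beat interval and writes the result to the mesh materials' BeatInterval scalar parameter.
; The InverseStrobe flag negates that value.
; BeginPlay applies a default strobe time, and the Blueprint leaves any animation to the material.
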(event `self.ReceiveBeginPlay`
  (`self.SetStrobeTime` 1.0))

(event `SetStrobeTime`
  (params (StrobeTime :type "Float (double-precision)" :default 1.0))
  (bind _mesh (`self.Mesh`))
  (bind _returnvalue (/ StrobeTime (`LightingTimerManager.BeatInterval` (`self.LightingTimerManager`))))
  (if (`self.InverseStrobe`)
    (`MeshComponent.SetScalarParameterValueOnMaterials` _mesh "BeatInterval" (* _returnvalue -1.0))
    (else
      (`MeshComponent.SetScalarParameterValueOnMaterials` _mesh "BeatInterval" _returnvalue))))

(fn `UserConstructionScript`)