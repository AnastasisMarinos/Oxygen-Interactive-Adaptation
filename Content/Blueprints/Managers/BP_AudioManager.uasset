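; BP_AudioManager runs the game's ending sequence when its final-line-started event fires.
; It binds to that event on BeginPlay, then waits a short delay before acting.
; It destroys all skeletal mesh actors, tells stage lights the game has ended, sets a strobe time on ceiling lights and makes the player character blink.
; After a longer delay it quits the game.
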(event `self.ReceiveBeginPlay`
  (add `self.OnFinalLineStarted` (delegate `OnFinalLineStarted_Event`)))

(event `OnFinalLineStarted_Event`
  (`KismetSystemLibrary.Delay` 7.5)
  (`|ExecutionSequence`
    (:`then_0`
      (bind _outactors (`GameplayStatics.GetAllActorsOfClass` "/Script/Engine.SkeletalMeshActor"))
      (for _array_element _outactors
        (`self.K2_DestroyActor` _array_element)))
    (:`then_1`
      (bind _outactors_2 (`GameplayStatics.GetAllActorsOfClass` "/Game/Blueprints/Lights/BP_StageLight.BP_StageLight_C"))
      (for _array_element_2 _outactors_2
        (`/Game/Blueprints/Lights/BP_StageLight.OnGameEnd` _array_element_2)))
    (:`then_2`
      (bind _outactors_3 (`GameplayStatics.GetAllActorsOfClass` "/Game/Blueprints/Lights/BP_CeilingLights.BP_CeilingLights_C"))
      (for _array_element_3 _outactors_3
        (`/Game/Blueprints/Lights/BP_CeilingLights.SetStrobeTime` _array_element_3 0.25)))
    (:`then_3`
      (bind _asbp_player_character (cast `/Game/Blueprints/Player/BP_PlayerCharacter` (`GameplayStatics.GetPlayerCharacter` 0)))
      (`PlayerCharacter.Blink` _asbp_player_character))
    (:`then_4`
      (`KismetSystemLibrary.Delay` 86.5)
      (`KismetSystemLibrary.QuitGame` (`GameplayStatics.GetPlayerController` 0) "Quit"))))

(fn `UserConstructionScript`)